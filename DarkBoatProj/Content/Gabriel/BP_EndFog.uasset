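; BP_EndFog is an end-of-game fog actor that rolls atmospheric fog in to close out play.
; On BeginPlay it registers itself with the game mode, then StartFog sets colour and start distance and waits a given play time.
; A timeline scaled to the roll time shrinks or alters the start distance, then a second timeline drives density offset as a fade.
; The end-game step currently only prints a debug message.
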(event `self.ReceiveBeginPlay`
  (message `/Game/Gamemodes/BPI_Gamemode.GiveFogRef` (`GameplayStatics.GetGameMode`) self))

(event `self.StartFog`
  (params (FogColour :type "LinearColor Structure") (StartDistance :type "Float (single-precision)") (PlayTimeBeforeFogBegin :type "Float (single-precision)") (FogRollTime :type "Float (single-precision)"))
  (bind _atmosphericfogcomponent (`self.AtmosphericFogComponent`))
  ;[1 1 1] Set Start Distance and Wait
  (`AtmosphericFogComponent.SetDefaultLightColor` _atmosphericfogcomponent FogColour)
  (`AtmosphericFogComponent.SetStartDistance` _atmosphericfogcomponent StartDistance)
  (`KismetSystemLibrary.Delay` PlayTimeBeforeFogBegin)
  ;[1 1 1] Start Fog Roll In
  (`TimelineComponent.SetPlayRate` (`self.Atmospheric Fog Timeline`) (/ 1.0 FogRollTime))
  (bind (_direction _start_dist_mult) (`Timeline|Atmospheric Fog Timeline` :!via `PlayFromStart`)
    (:`Update`
      (`AtmosphericFogComponent.SetStartDistance` _atmosphericfogcomponent (* _start_dist_mult (`self.Start Distance`))))
    (:`Finished`
      ;[1 1 1] Play End Fade To Black
      (bind (_direction_2 _start_distance) (`Timeline|EndFade` :!via `PlayFromStart`)
        (:`Update`
          (`AtmosphericFogComponent.SetDensityOffset` _atmosphericfogcomponent _start_distance))
        (:`Finished`
          ;[1 1 1] END GAME
          (`KismetSystemLibrary.PrintString` "Fog EndGame Triggered" true true (struct :`G` 0.66 :`B` 1.0 :`A` 1.0) 15.0))))))

(fn `UserConstructionScript`)